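; BP_Door is a door that swings open when the third-person character enters its Box trigger with a Puntaje score of at least five.
; The AbrirPuerta timeline yaws the Arrow component by lerping between open and close angles using its AnimPuerta track.
; With a lower score it shows an InterfazInteraccion widget, removed on leaving the box; nothing reverses the door.
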(event `self.Box.OnComponentBeginOverlap`
  (params (OverlappedComponent :type "PrimitiveComponent Object Reference") (OtherActor :type "Actor Object Reference") (OtherComp :type "PrimitiveComponent Object Reference") (OtherBodyIndex :type Integer) (bFromSweep :type Boolean) (SweepResult :type "HitResult Structure (by ref)"))
  (bind _asbp_third_person_character (cast `/Game/ThirdPerson/Blueprints/BP_ThirdPersonCharacter` OtherActor))
  (if (>= (`/Game/ThirdPerson/Blueprints/BP_ThirdPersonCharacter.Puntaje` _asbp_third_person_character) 5)
    (bind (_direction _animpuerta) (`Timeline|Abrir Puerta`)
      (:`Update`
        (`SceneComponent.K2_SetRelativeRotation` (`self.Arrow`) (`KismetMathLibrary.MakeRotator` 0.0 0.0 (`KismetMathLibrary.Lerp` (`self.AbrirPuerta`) (`self.CerrarPuerta`) _animpuerta)) false false)))
    (else
      (bind _returnvalue (`|CreateWidget` "/Game/Interfaces/InterfazInteraccion.InterfazInteraccion_C"))
      (bind _output_get (set `self.Interaccion` _returnvalue))
      (`UserWidget.AddToViewport` _output_get 0))))

(event `self.Box.OnComponentEndOverlap`
  (params (OverlappedComponent :type "PrimitiveComponent Object Reference") (OtherActor :type "Actor Object Reference") (OtherComp :type "PrimitiveComponent Object Reference") (OtherBodyIndex :type Integer))
  (bind _interaccion (`self.Interaccion`))
  (cast `/Game/ThirdPerson/Blueprints/BP_ThirdPersonCharacter` OtherActor)
  (`/Engine/EditorBlueprintResources/StandardMacros.IsValid` _interaccion
    (:`Is Valid`
      (`Widget.RemoveFromParent` _interaccion))))

(fn `UserConstructionScript`)